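; Prototype driving actor in _ZombieProto that moves a physics SphereCollision using Enhanced Input, adding IMC_Driving on BeginPlay.
; IA_Accelerate applies mass-independent force along the actor's forward vector, alongside a zero-torque call.
; IA_Move negates X, normalizes the input and scales by RollTorque, but uses only Y, transformed by the Scene component's relative transform, as torque.
; IA_Move also prints debug values; Tick and construction script are empty.
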(event `self.ReceiveBeginPlay`
  (`EnhancedInputSubsystemInterface.AddMappingContext` (pcsubsystem `EnhancedInputLocalPlayerSubsystem` (`GameplayStatics.GetPlayerController` 0)) "/Game/_ZombieProto/Input/IMC_Driving.IMC_Driving" 0 (struct)))

(event `self.ReceiveTick`
  (params (DeltaSeconds :type "Float (single-precision)")))

(event `EnhancedInput|/Game/_ZombieProto/Input/Actions/IA_Accelerate`
  (params (ActionValue :type "Float (double-precision)") (ElapsedSeconds :type "Float (double-precision)") (TriggeredSeconds :type "Float (double-precision)") (InputAction :type "InputAction Object Reference" :default "/Game/_ZombieProto/Input/Actions/IA_Accelerate.IA_Accelerate"))
  (:`Triggered`
    (`PrimitiveComponent.AddForce` (`self.SphereCollision`) (* (`self.GetActorForwardVector`) (`self.Acceleration`) ActionValue) "None" true)
    (`PrimitiveComponent.AddTorqueInRadians` (`self.SphereCollision`) (0.0 0.0 0.0) "None" false)))

(event `EnhancedInput|/Game/_ZombieProto/Input/Actions/IA_Move`
  (params (ActionValue :type "Vector2D Structure") (ElapsedSeconds :type "Float (double-precision)") (TriggeredSeconds :type "Float (double-precision)") (InputAction :type "InputAction Object Reference" :default "/Game/_ZombieProto/Input/Actions/IA_Move.IA_Move"))
  (bind _returnvalue (* ActionValue_X -1.0))
  (bind (_returnvalue_x _returnvalue_y) (`KismetMathLibrary.BreakVector2D` (* (`KismetMathLibrary.Normal2D` (`KismetMathLibrary.MakeVector2D` _returnvalue ActionValue_Y)) (`self.Roll Torque`))))
  (:`Triggered`
    (`KismetSystemLibrary.PrintString` (`KismetStringLibrary.Concat_StrStr` "ACTION VALUE X" (`KismetStringLibrary.Conv_DoubleToString` _returnvalue)))
    (`KismetSystemLibrary.PrintString` (`KismetStringLibrary.Concat_StrStr` "Y OUTPUT" "" (`KismetStringLibrary.Conv_DoubleToString` _returnvalue_y)))
    (`PrimitiveComponent.AddTorqueInRadians` (`self.SphereCollision`) (`KismetMathLibrary.TransformDirection` (`SceneComponent.GetRelativeTransform` (`self.Scene`)) (`KismetMathLibrary.MakeVector` 0.0 _returnvalue_y)) "None" false)))

(fn `UserConstructionScript`)