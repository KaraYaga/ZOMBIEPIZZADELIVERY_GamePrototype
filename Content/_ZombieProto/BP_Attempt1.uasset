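; Prototype physics car that hovers on four raycast suspension points, one per wheel, and pushes itself forward.
; Each tick, SuspensionCast traces down from every wheel and applies a compression-scaled spring force to CarBody, with no damping term.
; Grounded wheels also add a mass-scaled forward force driven by Acceleration.
; BeginPlay adds an input mapping context, but no input events exist and the Acceleration easing is unconnected.
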(event `self.ReceiveBeginPlay`
  ;[0.04688 1 0.2682 0.5] Event PLAY and TICK
  (`EnhancedInputSubsystemInterface.AddMappingContext` (pcsubsystem `EnhancedInputLocalPlayerSubsystem` (`GameplayStatics.GetPlayerController` 0)) null 0 (struct)))

(event `self.ReceiveTick`
  (params (DeltaSeconds :type "Float (single-precision)"))
  ;[0.04688 1 0.2682 0.5] Event PLAY and TICK
  (`self.SuspensionCast` (`self.FL_Wheel`))
  (`self.SuspensionCast` (`self.FR_Wheel`))
  (`self.SuspensionCast` (`self.BL_Wheel`))
  (`self.SuspensionCast` (`self.BR_Wheel`)))

(event `EnhancedInput|/Game/_ZombieProto/Input/Actions/IA_Accelerate`
  (params (ActionValue :type "Float (double-precision)") (ElapsedSeconds :type "Float (double-precision)") (TriggeredSeconds :type "Float (double-precision)") (InputAction :type "InputAction Object Reference" :default "/Game/_ZombieProto/Input/Actions/IA_Accelerate.IA_Accelerate"))
  ;[0.6264 0.4443 0.8542 0.5] ACCELERATION
)

(fn `SuspensionCast`
  (params (WheelComp :type "SceneComponent Object Reference"))
  (bind _returnvalue (`SceneComponent.K2_GetComponentLocation` WheelComp))
  (bind _car_body (`self.Car_Body`))
  ;[0.1142 0.7408 0.9531 0.5] Suspension
  (bind _outhit (`KismetSystemLibrary.LineTraceSingle` :`Start` _returnvalue :`End` (+ _returnvalue (0.0 0.0 -60.0)) :`TraceChannel` "TraceTypeQuery1" :`DrawDebugType` "ForOneFrame")) ; Line Trace from EACH wheel
  (bind (_bblockinghit _binitialoverlap _time _distance _location _impactpoint _normal _impactnormal _physmat _hitactor _hitcomponent _hitbonename _bonename _hititem _elementindex _faceindex _tracestart _traceend) (`GameplayStatics.BreakHitResult` _outhit))
  (if _bblockinghit
    (`PrimitiveComponent.AddForceAtLocation` (`self.Car_Body`) (* (- 1.0 (`KismetMathLibrary.NormalizeToRange` _distance 0.0 60.0)) (`KismetMathLibrary.GetDirectionUnitVector` _traceend _tracestart) (`self.Suspension Momentum`)) (`SceneComponent.K2_GetComponentLocation` (`local.WheelComp`)) "None")
    (`PrimitiveComponent.AddForceAtLocation` _car_body (* (`SceneComponent.GetForwardVector` _car_body) (`self.Vector Forward Force`) (`self.Acceleration`) (`PrimitiveComponent.GetMass` _car_body)) (`SceneComponent.K2_GetComponentLocation` (`local.WheelComp`)) "None") ; Force added to wheels
  ))

(fn `UserConstructionScript`)